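; Checkpoint actor that records a respawn location on the player's GAM1002_Character and shows its state through the Cube's material.
; The first Trigger overlap, without checking the overlapping actor, writes the checkpoint's location to CheckpointLoc, prints a message and switches to the enabled material.
; An IsActivated flag blocks repeat triggers until the character's Reset dispatcher, bound on BeginPlay, restores the disabled state.
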(event `Reset`
  ;[1 1 1] Reset
  (`PrimitiveComponent.SetMaterial` (`self.Cube`) 0 "/Game/disabled_M.disabled_M")
  (set `self.isActivated` false))

(event `self.ReceiveBeginPlay`
  ;[1 1 1] Set Player and Set Material
  (`|ExecutionSequence`
    (:`then_0`
      (set `self.isActivated` false)
      (bind _asgam1002_character (cast `/Game/Blueprints/GAM1002_Character` (`GameplayStatics.GetPlayerCharacter` 0)))
      (set `self.Player` _asgam1002_character)
      (`PrimitiveComponent.SetMaterial` (`self.Cube`) 0 "/Game/disabled_M.disabled_M"))
    (:`then_1`
      ;[1 1 1] Reset
      (add `/Game/Blueprints/GAM1002_Character.Reset` (`self.player`) (delegate `Reset`)))))

(event `self.Trigger.OnComponentBeginOverlap`
  (params (OverlappedComponent :type "PrimitiveComponent Object Reference") (OtherActor :type "Actor Object Reference") (OtherComp :type "PrimitiveComponent Object Reference") (OtherBodyIndex :type Integer) (bFromSweep :type Boolean) (SweepResult :type "HitResult Structure (by ref)"))
  ;[1 1 1] Trigger and Set Checkpoint and Material
  (if (not (`self.isActivated`))
    (bind _asgam1002_character (cast `/Game/Blueprints/GAM1002_Character` (`GameplayStatics.GetPlayerCharacter` 0)))
    (`KismetSystemLibrary.PrintString` "Checkpoint Reached")
    (set `/Game/Blueprints/GAM1002_Character.checkpointLoc` (`self.K2_GetActorLocation`) _asgam1002_character)
    (`PrimitiveComponent.SetMaterial` (`self.Cube`) 0 "/Game/enabled_M.enabled_M")
    (set `self.isActivated` true)))

(fn `UserConstructionScript`
  (`PrimitiveComponent.SetMaterial` (`self.Cube`) 0 "/Game/disabled_M.disabled_M"))