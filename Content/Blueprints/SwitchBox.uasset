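; SwitchBox is a one-shot trigger that activates when a pickupCube overlaps its Box component.
; The first cube overlap sets Switched, prints a debug message and broadcasts the SwitchBoxPressed dispatcher.
; On BeginPlay it binds to the GAM1002_Character player's Reset event, which clears Switched so the box can trigger again.
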(event `Reset`
  ;[1 1 1] Reset
  (set `self.switched` false))

(event `self.ReceiveBeginPlay`
  ;[1 1 1] Set Player
  (bind _asgam1002_character (cast `/Game/Blueprints/GAM1002_Character` (`GameplayStatics.GetPlayerCharacter` 0)))
  (set `self.player` _asgam1002_character)
  ;[1 1 1] Reset
  (add `/Game/Blueprints/GAM1002_Character.Reset` (`self.player`) (delegate `Reset`)))

(event `self.Box.OnComponentBeginOverlap`
  (params (OverlappedComponent :type "PrimitiveComponent Object Reference") (OtherActor :type "Actor Object Reference") (OtherComp :type "PrimitiveComponent Object Reference") (OtherBodyIndex :type Integer) (bFromSweep :type Boolean) (SweepResult :type "HitResult Structure (by ref)"))
  ;[1 1 1] Say Pressed
  (if (not (`self.Switched`))
    (cast `/Game/Blueprints/pickupCube` OtherActor)
    (set `self.Switched` true)
    (`KismetSystemLibrary.PrintString` "Switched")
    (`self.SwitchBoxPressed` self)))

(fn `UserConstructionScript`)