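; Physics cube pickup that the player carries by holding the Pickup input, with its section marked "Not Working".
; Entering Box shows a prompt widget and enables input, unless TopBox flags the player standing on the cube, in which case physics is frozen instead.
; Pickup disables physics, collision and gravity and attaches the actor to the player; release or leaving Box detaches and restores them.
; The player's Reset event returns the cube to its start location with zero rotation.
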(event `Reset`
  ;[1 1 1] Reset
  (`SceneComponent.K2_SetWorldLocation` (`self.Cube`) (`self.startLoc`) false false)
  (`SceneComponent.K2_SetWorldRotation` :`self` (`self.Cube`)))

(event `self.ReceiveBeginPlay`
  ;[1 1 1] Set Player and StartLoc
  (`|ExecutionSequence`
    (:`then_0`
      (bind _asgam1002_character (cast `/Game/Blueprints/GAM1002_Character` (`GameplayStatics.GetPlayerCharacter` 0)))
      (set `self.player` _asgam1002_character)
      (set `self.startLoc` (`SceneComponent.K2_GetComponentLocation` (`self.Cube`)))
      (bind _returnvalue (`|CreateWidget` "/Game/Test/activateUI.activateUI_C"))
      (set `self.activateUI` _returnvalue))
    (:`then_1`
      ;[1 1 1] Reset
      (add `/Game/Blueprints/GAM1002_Character.Reset` (`self.player`) (delegate `Reset`)))))

(event `self.Box.OnComponentBeginOverlap`
  (params (OverlappedComponent :type "PrimitiveComponent Object Reference") (OtherActor :type "Actor Object Reference") (OtherComp :type "PrimitiveComponent Object Reference") (OtherBodyIndex :type Integer) (bFromSweep :type Boolean) (SweepResult :type "HitResult Structure (by ref)"))
  ;[1 1 1] Trigger In Out
  (cast `/Game/Blueprints/GAM1002_Character` OtherActor)
  (`/Engine/EditorBlueprintResources/StandardMacros.DoOnce` false :!label _label
    (:`Completed`
      (`UserWidget.AddToViewport` (`self.activateUI`) 0)
      (if (`self.isColliding`)
        (`PrimitiveComponent.SetSimulatePhysics` (`self.Cube`) false)
        (else
          (`self.EnableInput` (`GameplayStatics.GetPlayerController` 0)))))))

(event `self.Box.OnComponentEndOverlap`
  (params (OverlappedComponent :type "PrimitiveComponent Object Reference") (OtherActor :type "Actor Object Reference") (OtherComp :type "PrimitiveComponent Object Reference") (OtherBodyIndex :type Integer))
  (bind _cube (`self.Cube`))
  ;[1 1 1] Trigger In Out
  (cast `/Game/Blueprints/GAM1002_Character` OtherActor)
  (`Widget.RemoveFromParent` (`self.activateUI`))
  (`self.DisableInput` (`GameplayStatics.GetPlayerController` 0))
  (`PrimitiveComponent.SetSimulatePhysics` (`self.Cube`) true)
  (`self.K2_DetachFromActor` "KeepWorld" "KeepWorld" "KeepWorld")
  (`PrimitiveComponent.SetCollisionEnabled` _cube "QueryAndPhysics")
  (`PrimitiveComponent.SetEnableGravity` _cube true)
  (goto _label :!via `Reset`))

(event `self.TopBox.OnComponentBeginOverlap`
  (params (OverlappedComponent :type "PrimitiveComponent Object Reference") (OtherActor :type "Actor Object Reference") (OtherComp :type "PrimitiveComponent Object Reference") (OtherBodyIndex :type Integer) (bFromSweep :type Boolean) (SweepResult :type "HitResult Structure (by ref)"))
  ;[1 1 1] Is Playing Standing on Cube
  (cast `/Game/Blueprints/GAM1002_Character` OtherActor)
  (set `self.isColliding` true))

(event `InputAction|Pickup`
  (params (Key :type "Key Structure"))
  (bind _cube (`self.Cube`))
  (bind _cube_2 (`self.Cube`))
  ;[1 1 1] Not Working
  (:`Pressed`
    (`|ExecutionSequence`
      (:`then_0`
        (`PrimitiveComponent.SetSimulatePhysics` _cube false)
        (`PrimitiveComponent.SetCollisionEnabled` _cube_2 "NoCollision")
        (`PrimitiveComponent.SetEnableGravity` _cube_2 false)
        (`Widget.RemoveFromParent` (`self.activateUI`)))
      (:`then_1`
        (`self.K2_AttachToActor` (`self.player`) "None" "KeepWorld" "KeepWorld" "KeepWorld" false))))
  (:`Released`
    (`|ExecutionSequence`
      (:`then_0`
        (`self.K2_DetachFromActor` "KeepWorld" "KeepWorld" "KeepWorld"))
      (:`then_1`
        (`PrimitiveComponent.SetSimulatePhysics` _cube true)
        (`PrimitiveComponent.SetCollisionEnabled` _cube_2 "QueryAndPhysics")
        (`PrimitiveComponent.SetEnableGravity` _cube_2 true)
        (goto _label :!via `Reset`)))))

(event `self.TopBox.OnComponentEndOverlap`
  (params (OverlappedComponent :type "PrimitiveComponent Object Reference") (OtherActor :type "Actor Object Reference") (OtherComp :type "PrimitiveComponent Object Reference") (OtherBodyIndex :type Integer))
  ;[1 1 1] Is Playing Standing on Cube
  (cast `/Game/Blueprints/GAM1002_Character` OtherActor)
  (set `self.isColliding` false))

(fn `UserConstructionScript`)