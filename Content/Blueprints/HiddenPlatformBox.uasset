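; Hidden platform actor that stays invisible and non-collidable until its linked switch box is pressed.
; On BeginPlay it hides Cube1, then binds to the SwitchBox pressed event and to the GAM1002_Character's Reset event.
; A press from the matching switch makes the cube visible and solid, and the player's reset hides it again.
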(event `Reset`
  (bind _cube1 (`self.Cube1`))
  ;[1 1 1] Reset
  (`PrimitiveComponent.SetCollisionEnabled` _cube1 "NoCollision")
  (`SceneComponent.SetVisibility` _cube1 false false))

(event `self.ReceiveBeginPlay`
  (bind _cube1 (`self.Cube1`))
  ;[1 1 1] Get Player, Set Inactive
  (bind _asgam1002_character (cast `/Game/Blueprints/GAM1002_Character` (`GameplayStatics.GetPlayerCharacter` 0)))
  (set `self.player` _asgam1002_character)
  (`|ExecutionSequence`
    (:`then_0`
      (`PrimitiveComponent.SetCollisionEnabled` _cube1 "NoCollision" :!label _label)
      (`SceneComponent.SetVisibility` _cube1 false false))
    (:`then_1`
      (add `/Game/Blueprints/SwitchBox.SwitchBoxPressed` (`self.switchBox`) (delegate `ShowPlatform`))
      (goto _label))
    (:`then_2`
      ;[1 1 1] Reset
      (add `/Game/Blueprints/GAM1002_Character.Reset` (`self.player`) (delegate `Reset`)))))

(event `ShowPlatform`
  (params (SwitchBox :type "/Game/Blueprints/SwitchBox Object Reference"))
  (bind _cube1 (`self.Cube1`))
  ;[1 1 1] Get Player, Set Inactive
  (if (== SwitchBox (`self.switchBox`))
    (bind _output_get (set `self.isEnabled` true))
    (if _output_get
      (`PrimitiveComponent.SetCollisionEnabled` _cube1 "QueryAndPhysics")
      (`SceneComponent.SetVisibility` _cube1 true false)
      (else
        (`PrimitiveComponent.SetCollisionEnabled` _cube1 "NoCollision")
        (`SceneComponent.SetVisibility` _cube1 false false)))))

(fn `UserConstructionScript`)