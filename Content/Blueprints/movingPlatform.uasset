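; Moving platform actor that travels back and forth between the locations of two referenced actors, StartLoc and EndLoc.
; It snaps to StartLoc on BeginPlay, then each Tick calls ToEnd or ToStart depending on the Ended flag.
; Both events move it by constant-speed interpolation scaled by MovementMultiplier, without sweep.
; After a zero-length delay, they flip Ended once the platform is within a small tolerance of its target.
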(event `self.ReceiveBeginPlay`
  (`self.K2_SetActorLocation` (`self.K2_GetActorLocation` (`self.startLoc`))))

(event `toEnd`
  (bind _returnvalue (`self.K2_GetActorLocation` (`self.endLoc`)))
  (bind _returnvalue_2 (`self.K2_GetActorLocation` self))
  (`self.K2_SetActorLocation` self (`KismetMathLibrary.VInterpTo_Constant` _returnvalue_2 _returnvalue (`GameplayStatics.GetWorldDeltaSeconds`) (* (`self.MovementMultiplier`) 20.0)) false false)
  (`KismetSystemLibrary.Delay` 0.0)
  (if (== _returnvalue_2 _returnvalue :`ErrorTolerance` 50.0)
    (set `self.ended` true)))

(event `self.ReceiveTick`
  (params (DeltaSeconds :type "Float (single-precision)"))
  (if (`self.ended`)
    (`self.toStart`)
    (else
      (`self.toEnd`))))

(event `toStart`
  (bind _returnvalue (`self.K2_GetActorLocation` self))
  (bind _returnvalue_2 (`self.K2_GetActorLocation` (`self.startLoc`)))
  (`self.K2_SetActorLocation` self (`KismetMathLibrary.VInterpTo_Constant` _returnvalue _returnvalue_2 (`GameplayStatics.GetWorldDeltaSeconds`) (* (`self.MovementMultiplier`) 20.0)) false false)
  (`KismetSystemLibrary.Delay` 0.0)
  (if (== _returnvalue _returnvalue_2 :`ErrorTolerance` 50.0)
    (set `self.ended` false)))

(fn `UserConstructionScript`)